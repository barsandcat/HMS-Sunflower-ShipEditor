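; BP_MyGameMode is a game mode that shows a part browser UI and tracks the current state of an editing workflow.
; On BeginPlay it creates WBP_PartBrowser, stores it and adds it to the viewport.
; Its Cancel and SelectPart functions follow a state pattern, forwarding to EditState and replacing it with the returned state.
; SelectPart currently passes a fixed zero argument.
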(event EventBeginPlay
  (bind _returnvalue (UserInterface|CreateWidget "/Game/WBP_PartBrowser.WBP_PartBrowser_C"))
  (bind _output_get (Variables|Default|SetPartBrowser _returnvalue))
  (UserInterface|Viewport|AddtoViewport _output_get 0))

(event EventTick
  (params (DeltaSeconds :type Float%20%28single-precision%29)))

(fn ConstructionScript)

(fn Cancel
  (bind _returnvalue (Class|EditStateInterface|Cancel (Variables|Default|GetEditState)))
  (Variables|Default|SetEditState _returnvalue))

(fn SelectPart
  (bind _returnvalue (Class|EditStateInterface|SelectPart (Variables|Default|GetEditState)))
  (Variables|Default|SetEditState _returnvalue))